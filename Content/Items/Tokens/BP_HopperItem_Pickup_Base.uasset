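; Base pickup actor for Hopper tokens (coin, jump, punch), collected when a Player-tagged character overlaps it.
; On overlap it disables collision and adds the item to the player controller's inventory; coins also bump and check the controller's coin count.
; Jump and punch tokens set matching ability flags on the character, with a sound per type.
; A timeline shrinks the flipbook toward the player, then destroys the actor.
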(event `self.CollectCollision.OnComponentBeginOverlap`
  (params (OverlappedComponent :type "PrimitiveComponent Object Reference") (OtherActor :type "Actor Object Reference") (OtherComp :type "PrimitiveComponent Object Reference") (OtherBodyIndex :type Integer) (bFromSweep :type Boolean) (SweepResult :type "HitResult Structure (by ref)"))
  (if (`self.ActorHasTag` OtherActor "Player")
    (bind _ascharacter (cast `Character` OtherActor))
    (bind _output_get (set `self.PlayerCollecting` _ascharacter))
    (`PrimitiveComponent.SetCollisionEnabled` (`self.CollectCollision`) "NoCollision")
    (`self.GiveItem`)
    (bind _asbp_hopper_player_controller (cast `/Game/Blueprints/Core/BP_HopperPlayerController` (`Pawn.GetController` _output_get)))
    (if (== (`self.ItemType`) "/Game/Items/Tokens/Token_Coin.Token_Coin")
      (`/Engine/EditorBlueprintResources/StandardMacros.IncrementInt` (`/Game/Blueprints/Core/BP_HopperPlayerController.CurrentCointCount` _asbp_hopper_player_controller)
        (:`  `
          (`/Game/Blueprints/Core/BP_HopperPlayerController.CheckCoinCoint` _asbp_hopper_player_controller)
          (`GameplayStatics.PlaySound2D` "/Game/Interface_And_Item_Sounds/Cues/Coins_02_Cue.Coins_02_Cue" 1.0 1.0 0.0 null null))))))

(event `GiveItem`
  (bind _playercollecting (`self.PlayerCollecting`))
  (`/Engine/EditorBlueprintResources/StandardMacros.IsValid` _playercollecting
    (:`Is Valid`
      (bind _asbp_hopper_player_controller (cast `/Game/Blueprints/Core/BP_HopperPlayerController` (`Pawn.GetController` _playercollecting)))
      (`HopperPlayerController.AddInventoryItem` _asbp_hopper_player_controller (`self.ItemType`) (`self.Count`) 1)
      (`self.AnimateCollection`)
      (bind _asbp_hopper_base_character (cast `/Game/Blueprints/Characters/BP_HopperBaseCharacter` (`Controller.K2_GetPawn` _asbp_hopper_player_controller)))
      (if (== (`self.ItemType`) "/Game/Items/Tokens/Token_Jump.Token_Jump")
        (set `/Game/Blueprints/Characters/BP_HopperBaseCharacter.IsTokenJump` true _asbp_hopper_base_character)
        (`GameplayStatics.PlaySound2D` "/Game/Interface_And_Item_Sounds/Cues/Special_Powerup_08_Cue.Special_Powerup_08_Cue" 1.0 1.0 0.0 null null)
        (elif (== (`self.ItemType`) "/Game/Items/Tokens/Token_Punch.Token_Punch")
          (set `HopperBaseCharacter.bCanPunchToken` true _asbp_hopper_base_character)
          (`GameplayStatics.PlaySound2D` "/Game/Interface_And_Item_Sounds/Cues/Special_Powerup_09_Cue.Special_Powerup_09_Cue" 1.0 1.0 0.0 null null))))))

(event `AnimateCollection`
  (set `self.FlipbookWorldLocation` (`SceneComponent.K2_GetComponentLocation` (`self.PaperFlipbook`)))
  (bind (_direction _alpha) (`Timeline|Animate`)
    (:`Update`
      (`SceneComponent.SetRelativeScale3D` (`self.PaperFlipbook`) (`KismetMathLibrary.VLerp` (`SceneComponent.K2_GetComponentScale` (`self.PaperFlipbook`)) (0.0 0.0 0.0) _alpha))
      (`SceneComponent.K2_SetWorldLocation` (`self.PaperFlipbook`) (`KismetMathLibrary.VLerp` (`self.FlipbookWorldLocation`) (`self.K2_GetActorLocation` (`self.PlayerCollecting`)) _alpha) false true))
    (:`Finished`
      (`self.K2_DestroyActor`))))

(fn `UserConstructionScript`)