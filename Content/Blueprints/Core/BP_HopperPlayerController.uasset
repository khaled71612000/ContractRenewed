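; BP_HopperPlayerController is the player controller for a Hopper game, owning the HUD and the coin-based win check.
; On BeginPlay it creates WBP_HopperHUD, stores it as InventoryUI and adds it to the viewport.
; CheckCoinCoint, which has no caller in this graph, compares the current coin count to the target.
; Once the target is met, it shows BP_GameWon, enables the mouse cursor and pauses the game.
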(event `self.ReceiveBeginPlay`
  (`self.SetupUI`))

(event `SetupUI`
  (bind _returnvalue (`|CreateWidget` "/Game/Widgets/WBP_HopperHUD.WBP_HopperHUD_C" self self))
  (bind _output_get (set `self.InventoryUI` _returnvalue))
  (`UserWidget.AddToViewport` _output_get 0))

(event `CheckCoinCoint`
  (if (>= (`self.CurrentCointCount`) (`self.TargetCointCount`))
    (bind _returnvalue (`|CreateWidget` "/Game/Widgets/BP_GameWon.BP_GameWon_C"))
    (`UserWidget.AddToViewport` _returnvalue 0)
    (set `PlayerController.bShowMouseCursor` true (`GameplayStatics.GetPlayerController` 0))
    (`GameplayStatics.SetGamePaused` true)))

(fn `UserConstructionScript`)