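; Player character for the hopper game, apparently its hard variant, with camera-relative movement and a flipbook sprite that freezes mid-jump.
; When IsTokenJump is set, consecutive jumps within a short landing window escalate jump power through three tiers, with squash-and-stretch calls.
; Spawning locks input while a timeline drives a material parameter collection effect, then flickers the sprite.
; Overlapping a KillZVolume pauses the game and shows the game-over widget.
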(event `InputAxis|Up`
  (params (AxisValue :type "Float (single-precision)"))
  ;[0.006795 0 1] Movement
  (`self.AddMovementInput` (`SceneComponent.GetForwardVector` (`self.Camera_0`)) AxisValue))

(event `InputAxis|Right`
  (params (AxisValue :type "Float (single-precision)"))
  ;[0.006795 0 1] Movement
  (`self.AddMovementInput` (`SceneComponent.GetRightVector` (`self.Camera_0`)) AxisValue))

(event `InputAxis|LookUp`
  (params (AxisValue :type "Float (single-precision)"))
  ;[0.006795 0 1] Movement
  (`self.AddControllerPitchInput` AxisValue))

(event `InputAxis|Turn`
  (params (AxisValue :type "Float (single-precision)"))
  ;[0.006795 0 1] Movement
  (`self.AddControllerYawInput` AxisValue))

(event `InputAction|Jump`
  (params (Key :type "Key Structure"))
  ;[0.006795 0 1] Movement
  (:`Pressed`
    (`self.Jump`)
    (`GameplayStatics.PlaySoundAtLocation` "/Game/Interface_And_Item_Sounds/Cues/retro-jump-3-236683.retro-jump-3-236683" (`self.K2_GetActorLocation`) (struct) 1.0 1.0 0.0 null null null null)
    (if (`NavMovementInterface.IsMovingOnGround` (`self.CharacterMovement`))
      (`self.JumpSqueeze`))))

(event `self.OnJumped`
  (set `CharacterMovementComponent.bNotifyApex` true (`self.CharacterMovement`))
  (`PaperFlipbookComponent.SetPlayRate` (`self.Sprite`) 0.0)
  (`PaperFlipbookComponent.SetPlaybackPositionInFrames` (`self.Sprite`) 0 true)
  (`/Engine/EditorBlueprintResources/StandardMacros.IncrementInt` (`self.JumpCounter`)
    (:`  `
      (`KismetSystemLibrary.K2_ClearAndInvalidateTimerHandle` (`self.JumpReset`)))))

(event `self.OnLanded`
  (params (Hit :type "HitResult Structure (by ref)"))
  (`PaperFlipbookComponent.SetPlayRate` (`self.Sprite`) 1.0)
  (set `CharacterMovementComponent.GravityScale` 2.8 (`self.CharacterMovement`))
  (if (> (`self.JumpCounter`) 2)
    (set `self.JumpCounter` 0))
  (`self.ModifyJumpPower`)
  (bind _returnvalue (`KismetSystemLibrary.K2_SetTimerDelegate` (delegate `ResetJumpPower`) 0.2))
  (set `self.JumpReset` _returnvalue)
  (`self.LandSquish`))

(event `ModifyJumpPower`
  (if (`self.IsTokenJump`)
    (set `CharacterMovementComponent.JumpZVelocity` (select `int` (`self.JumpCounter`) :`0` 1000.0 :`1` 1400.0 :`2` 1800.0 :!type "Float (single-precision)") (`self.CharacterMovement`))
    (else
      (set `CharacterMovementComponent.JumpZVelocity` 1000.0 (`self.CharacterMovement`)))))

(event `ResetJumpPower`
  (set `CharacterMovementComponent.JumpZVelocity` 1000.0 (`self.CharacterMovement`))
  (set `self.JumpCounter` 0))

(event `self.CapsuleComponent.OnComponentBeginOverlap`
  (params (OverlappedComponent :type "PrimitiveComponent Object Reference") (OtherActor :type "Actor Object Reference") (OtherComp :type "PrimitiveComponent Object Reference") (OtherBodyIndex :type Integer) (bFromSweep :type Boolean) (SweepResult :type "HitResult Structure (by ref)"))
  (cast `KillZVolume` OtherActor)
  (bind _returnvalue (`|CreateWidget` "/Game/Widgets/BP_GameOver.BP_GameOver_C"))
  (`UserWidget.AddToViewport` _returnvalue 0)
  (set `PlayerController.bShowMouseCursor` true (`GameplayStatics.GetPlayerController` 0))
  (`GameplayStatics.SetGamePaused` true))

(event `self.ReceiveBeginPlay`
  (`parent.ReceiveBeginPlay`)
  (`Controller.SetControlRotation` (`self.GetController`) (`KismetMathLibrary.MakeRotator` 0.0 -20.0))
  (`self.DisableInput` (`GameplayStatics.GetPlayerController` 0))
  (`KismetMaterialLibrary.SetVectorParameterValue` "/Game/Material/WorldDEres/PC_Control.PC_Control" "Location" (`KismetMathLibrary.Conv_VectorToLinearColor` (`SceneComponent.K2_GetComponentLocation` (`self.Sprite`))))
  (bind (_direction _newtrack_0) (`Timeline|Timeline_0`)
    (:`Update`
      (`KismetMaterialLibrary.SetScalarParameterValue` "/Game/Material/WorldDEres/PC_Control.PC_Control" "Amount" _newtrack_0))
    (:`Finished`
      (`self.StartSpriteFlicker`)
      (`KismetSystemLibrary.Delay` 2.0)
      (`self.StopSpriteFlicker`)
      (`self.EnableInput` (`GameplayStatics.GetPlayerController` 0)))))

(fn `UserConstructionScript`)