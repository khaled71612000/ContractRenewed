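; BP_HopperEnemy is a sprite-based enemy character that players can squash and that reacts to its death.
; A tagged player's qualifying capsule hit launches that player upward and activates the GA_Squash ability.
; HandleSquashed disables collision and flattens the sprite.
; On death, the authority stops AI movement and logic, tints the sprite red, then after a delay spawns a pop effect and destroys the actor.
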(event `self.ReceiveBeginPlay`
  (`parent.ReceiveBeginPlay`))

(event `self.CapsuleComponent.OnComponentHit`
  (params (HitComponent :type "PrimitiveComponent Object Reference") (OtherActor :type "Actor Object Reference") (OtherComp :type "PrimitiveComponent Object Reference") (NormalImpulse :type "Vector Structure") (Hit :type "HitResult Structure (by ref)"))
  ;[1 0.121 0] Check if Squashed
  (if (and (`HopperBlueprintFunctionLibrary.IsSquashingHit` (`self.GetVelocity` OtherActor) 0.1) (`self.ActorHasTag` OtherActor "Player"))
    (`|ExecutionSequence`
      (:`then_0`
        (bind _asbp_hopper_player_character_hard (cast `/Game/Blueprints/Characters/BP_HopperPlayerCharacterHard` OtherActor))
        (`self.LaunchCharacter` _asbp_hopper_player_character_hard (0.0 0.0 400.0) false false)
        (`KismetSystemLibrary.PrintString` "LAUNCH"))
      (:`then_1`
        (`AbilitySystemComponent.TryActivateAbilityByClass` (`self.AbilitySystemComponent`) "/Game/Blueprints/Abilities/GA_Squash.GA_Squash_C" true)))))

(event `self.OnDeath`
  (bind _returnvalue (`AIBlueprintHelperLibrary.GetAIController` self))
  (bind _braincomponent (`AIController.BrainComponent` _returnvalue))
  ;[0 0 0] Death
  (`/Engine/EditorBlueprintResources/ActorMacros.Switch Has Authority`
    (:`Authority`
      (`|ExecutionSequence`
        (:`then_0`
          (`KismetSystemLibrary.K2_SetTimerDelegate` (delegate `PlayDeathAnimation`) 1.0))
        (:`then_1`
          (`/Engine/EditorBlueprintResources/StandardMacros.IsValid` _returnvalue
            (:`Is Valid`
              (`Controller.StopMovement` _returnvalue)
              (`/Engine/EditorBlueprintResources/StandardMacros.IsValid` _braincomponent
                (:`Is Valid`
                  (`BrainComponent.StopLogic` _braincomponent "Enemy has been killed."))))))
        (:`then_2`
          (`self.SetSpriteColor`))))))

(event `SetSpriteColor`
  ;[0 0 0] Death
  (`PaperFlipbookComponent.SetSpriteColor` (`self.Sprite`) (struct :`R` 1.0 :`G` 0.182292 :`B` 0.182292 :`A` 1.0)))

(event `PlayDeathAnimation`
  ;[0 0 0] Death
  (`NiagaraFunctionLibrary.SpawnSystemAtLocation` "/Game/FX/N_Pop.N_Pop" (`self.K2_GetActorLocation`))
  (`/Engine/EditorBlueprintResources/ActorMacros.Switch Has Authority`
    (:`Authority`
      (`self.DelayedDestroy`))))

(event `HandleSquashed`
  ;[0.8618 0 1] Squashed
  (`|ExecutionSequence`
    (:`then_0`
      (`PrimitiveComponent.SetCollisionEnabled` (`self.CapsuleComponent`) "NoCollision"))
    (:`then_1`
      (`self.SquashSprite`))))

(event `SquashSprite`
  (bind _sprite (`self.Sprite`))
  ;[0.8618 0 1] Squashed
  (`SceneComponent.SetRelativeScale3D` _sprite (/ (`SceneComponent.RelativeScale3D` _sprite) (1.0 1.0 2.0)))
  (`SceneComponent.K2_SetRelativeLocation` _sprite (0.0 0.0 -35.0) false true))

(event `DelayedDestroy`
  ;[0 0 0] Death
  (`self.K2_DestroyActor`))

(fn `UserConstructionScript`
  (`parent.UserConstructionScript`))