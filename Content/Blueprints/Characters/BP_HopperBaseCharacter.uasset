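; Base sprite character for Hopper, providing shared movement feedback, health bar updates and death triggering.
; Bound events spawn dust on footsteps and raise gravity at the jump apex for a faster fall.
; Health changes update the widget through a ShowHealthBar server event and call OnDeath at zero health.
; Timelines squash and stretch the sprite for jumps and landings, and a looping timer drives visibility flicker.
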(event `self.ReceiveBeginPlay`
  (add `self.OnFootstepTaken` (delegate `self.OnFootstep`))
  (add `self.OnReachedJumpApex` (delegate `ModifyGravity`))
  (set `self.BaseScale` (`SceneComponent.RelativeScale3D` (`self.Sprite`))))

(event `ModifyGravity`
  (set `CharacterMovementComponent.GravityScale` 5.0 (`self.CharacterMovement`)))

(event `self.OnFootstep`
  (bind _returnvalue (`self.K2_GetActorLocation`))
  ;[0 0 0] Footstep FX
  (`KismetSystemLibrary.LineTraceSingle` _returnvalue (+ _returnvalue (* (`self.GetActorUpVector`) -200.0)) "TraceTypeQuery1")
  (`NiagaraFunctionLibrary.SpawnSystemAtLocation` "/Game/FX/N_Poof_Dust.N_Poof_Dust" (- _returnvalue (0.0 0.0 75.0))))

(event `self.OnHealthChanged`
  (params (DeltaValue :type "Float (single-precision)") (EventTags :type "GameplayTagContainer Structure (by ref)"))
  ;[1 0 0.4329] On Health Changed
  (`self.ShowHealthBar_Server` (`self.GetHealth`))
  (if (not (`self.IsAlive`))
    (`self.OnDeath`)))

(event `ShowHealthBar_Server`
  (params (`Authority Health` :type "Float (double-precision)"))
  (bind _returnvalue (/ `Authority Health` (`self.GetMaxHealth`)))
  ;[1 0.2396 0.2396] Show Health Bar
  (bind _aswbp_health (cast `/Game/Widgets/WBP_Health` (`WidgetComponent.GetUserWidgetObject` (`self.HealthWidget`))))
  (`/Game/Widgets/WBP_Health.SetProgress` _aswbp_health _returnvalue)
  (`/Engine/EditorBlueprintResources/StandardMacros.DoOnce` false
    (:`Completed`
      (`Widget.SetVisibility` _aswbp_health (select `bool` (<= _returnvalue 1.0) :`false` "Hidden" :`true` "Visible" :!type "ESlateVisibility Enum")))))

(event `JumpSqueeze`
  (bind (_direction _alpha) (`Timeline|JumpSqueezeAnim` :!via `PlayFromStart`)
    (:`Update`
      (`SceneComponent.SetRelativeScale3D` (`self.Sprite`) (`KismetMathLibrary.VLerp` (`self.BaseScale`) (* (`self.BaseScale`) (`self.JumpSqueezeFactor`)) _alpha)))))

(event `LandSquish`
  (bind (_direction _alpha) (`Timeline|LandSquishAnim` :!via `PlayFromStart`)
    (:`Update`
      (`SceneComponent.SetRelativeScale3D` (`self.Sprite`) (`KismetMathLibrary.VLerp` (`self.BaseScale`) (* (`self.BaseScale`) (`self.LandSquishFactor`)) _alpha)))))

(fn `IsAlive`
  (returns (Return :type Boolean))
  (return (> (`self.GetHealth`) 0.0)))

(fn `StartSpriteFlicker`
  (bind _returnvalue (`KismetSystemLibrary.K2_SetTimerDelegate` (`|CreateDelegate` :!event `ToggleSpriteFlicker`) (`self.FlickerInterval`) true))
  (set `self.SpriteFlicker` _returnvalue))

(fn `StopSpriteFlicker`
  (`KismetSystemLibrary.K2_ClearAndInvalidateTimerHandle` (`self.SpriteFlicker`))
  (`SceneComponent.SetVisibility` (`self.Sprite`) true false))

(fn `ToggleSpriteFlicker`
  (`SceneComponent.SetVisibility` (`self.Sprite`) (not (`SceneComponent.bVisible` (`self.Sprite`))) true))

(fn `UserConstructionScript`)